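; Enemy spawner for a tower defence game that spawns queued enemy classes at its own transform.
; AddEnemyToQueue spawns immediately when no BP_Base actor overlaps its sphere, and a looping timer also pops the queue periodically.
; It binds to each enemy's destruction, with a death handler that notifies the game mode.
; The game mode's wave-end event sets IsOn from the upcoming wave and RoundActivated, though spawning here never checks it.
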(event `self.ReceiveBeginPlay`
  (`KismetSystemLibrary.K2_SetTimerDelegate` (delegate `TryToSwawn`) 2.0 true)
  (bind _asbp_tower_defence_aigame_mode_base (cast `/Game/GameMode/BP_TowerDefenceAIGameModeBase` (`GameplayStatics.GetGameMode`)))
  (bind _output_get (set `self.As BP Tower Defence AIGame Mode Base` _asbp_tower_defence_aigame_mode_base))
  (add `/Game/GameMode/BP_TowerDefenceAIGameModeBase.OnEndWave` _output_get (delegate `On End WAve`)))

(event `TryToSwawn`
  (`self.SpawnEnemy`))

(event `On End WAve`
  (set `self.isOn` (>= (+ (`/Game/GameMode/BP_TowerDefenceAIGameModeBase.WaveNumber` (`self.As BP Tower Defence AIGame Mode Base`)) 1) (`self.RoundActivated`))))

(event `OnEnemyDeath`
  (params (DestroyedActor :type "Actor Object Reference"))
  (bind _asbp_tower_defence_aigame_mode_base (cast `/Game/GameMode/BP_TowerDefenceAIGameModeBase` (`GameplayStatics.GetGameMode`)))
  (`/Game/GameMode/BP_TowerDefenceAIGameModeBase.OnEnemyDeath` _asbp_tower_defence_aigame_mode_base))

(fn `AddEnemyToQueue`
  (params (EnemyClass :type "/Game/AI/BP_Base Class Reference (by ref)"))
  ;[1 1 1] Add Enemy to queue
  (`KismetArrayLibrary.Array_Add` (`self.EnemyQueue`) EnemyClass)
  (if (not (`KismetArrayLibrary.Array_IsValidIndex` (`PrimitiveComponent.GetOverlappingActors` (`self.Sphere`) "/Game/AI/BP_Base.BP_Base_C")))
    (`self.SpawnEnemy`)))

(fn `SpawnEnemy`
  (returns (Succsess :type Boolean))
  (if (`KismetArrayLibrary.Array_IsValidIndex` (`self.EnemyQueue`))
    (bind _returnvalue (`|SpawnActorFromClass` (`|GetArrayItem` (`self.EnemyQueue`)) (`self.GetTransform`) "AdjustIfPossibleButAlwaysSpawn" "MultiplyWithRoot" null null))
    (add `self.OnDestroyed` _returnvalue (`|CreateDelegate` :!event `OnEnemyDeath`))
    (`KismetArrayLibrary.Array_Remove` (`self.EnemyQueue`))
    (return true)
    (else
      (return false))))

(fn `UserConstructionScript`)