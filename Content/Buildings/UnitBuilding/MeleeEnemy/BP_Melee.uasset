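; BP_Melee is an AI-controlled melee enemy unit that damages the target held by its AI_Unit controller.
; On BeginPlay it stores its spawn location, and every Tick it calls FireAt to read the controller's Enemy.
; For a valid target it draws a debug line trace from FirePoint and applies fixed damage each frame, regardless of the trace result or distance.
; A BP_Bullet spawn node is left unconnected.
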(event `self.ReceiveBeginPlay`
  (set `self.SpawnLocation` (`self.K2_GetActorLocation`)))

(event `self.ReceiveTick`
  (params (DeltaSeconds :type "Float (single-precision)"))
  (`self.FireAt`))

(event `FireAt`
  (bind _asai_unit (cast `/Game/Buildings/UnitBuilding/AI_Unit` (`AIBlueprintHelperLibrary.GetAIController` self)))
  (set `self.CurrantTarget` (`/Game/Buildings/UnitBuilding/AI_Unit.Enemy` _asai_unit))
  (`/Engine/EditorBlueprintResources/StandardMacros.IsValid` (`self.CurrantTarget`)
    (:`Is Valid`
      (`KismetSystemLibrary.LineTraceSingle` :`Start` (`SceneComponent.K2_GetComponentLocation` (`self.FirePoint`)) :`End` (`self.K2_GetActorLocation` (`self.CurrantTarget`)) :`TraceChannel` "TraceTypeQuery1" :`DrawDebugType` "ForDuration")
      (`GameplayStatics.ApplyDamage` (`self.CurrantTarget`) 2.0))))

(fn `UserConstructionScript`)