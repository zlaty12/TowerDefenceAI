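; AI controller for BP_Turret that runs the BT_Turret behavior tree on possession and manages the turret's targets.
; Sight perception adds sensed actors to a candidate list and removes lost ones, clearing the current target if it matches.
; A select function picks a random candidate, writes it to the turret and Blackboard, and reports success.
; A cannon look-at tracking function exists but is not wired to run in the event graph.
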(event `self.ReceivePossess`
  (params (PossessedPawn :type "Pawn Object Reference"))
  (bind _asbp_turret (cast `/Game/Buildings/Turret/BP_Turret` PossessedPawn))
  (set `self.As BP Turret` _asbp_turret)
  (`self.RunBehaviorTree` "/Game/Buildings/Turret/Behavior/BT_Turret.BT_Turret"))

(event `self.ReceiveTick`
  (params (DeltaSeconds :type "Float (single-precision)")))

(event `self.AIPerception.OnTargetPerceptionUpdated`
  (params (Actor :type "Actor Object Reference") (Stimulus :type "AIStimulus Structure"))
  (bind _returnvalue (`AIPerceptionSystem.GetSenseClassForStimulus` Stimulus))
  (if (== _returnvalue "/Script/AIModule.AISense_Sight")
    (if (`.bSuccessfullySensed` (break `AIStimulus` Stimulus))
      (`KismetArrayLibrary.Array_AddUnique` (`self.TargetActors`) Actor)
      (else
        (`self.RemmoveTargetActor` Actor)))))

(fn `ChooseTargetActor`
  (returns (SelectedActor :type "Actor Object Reference"))
  (if (`KismetArrayLibrary.Array_IsNotEmpty` (`self.TargetActors`))
    (bind _output_get (set `self.TargetActorToAimAt` (`KismetArrayLibrary.Array_Random` (`self.TargetActors`))))
    (return _output_get)
    (else
      (return null))))

(fn `Controller_TurretSelectTarget`
  (returns (IsTargetSet :type Boolean))
  (bind _selectedactor (`self.ChooseTargetActor`))
  (`/Engine/EditorBlueprintResources/StandardMacros.IsValid` _selectedactor
    (:`Is Valid`
      (`self.SetTargetActor` _selectedactor)
      (return true))
    (:`Is Not Valid`
      (return false))))

(fn `HandleTrackNPC`
  (bind _cannon (`/Game/Buildings/Turret/BP_Turret.CAnnon` (`self.As BP Turret`)))
  (if (`/Game/Buildings/Turret/BP_Turret.IsAiming` (`self.As BP Turret`))
    (`SceneComponent.K2_SetWorldRotation` _cannon (`KismetMathLibrary.FindLookAtRotation` (`SceneComponent.K2_GetComponentLocation` _cannon) (`SceneComponent.K2_GetComponentLocation` (`Actor.RootComponent` (`/Game/Buildings/Turret/BP_Turret.CurrantTarget` (`self.As BP Turret`))))) false false)))

(fn `RemmoveTargetActor`
  (params (TargetActor :type "Actor Object Reference (by ref)"))
  (if (== TargetActor (`/Game/Buildings/Turret/BP_Turret.CurrantTarget` (`self.As BP Turret`)))
    (set `/Game/Buildings/Turret/BP_Turret.CurrantTarget` null (`self.As BP Turret`))
    (`BlackboardComponent.ClearValue` (`self.Blackboard`) "CurrantTarget"))
  (`KismetArrayLibrary.Array_RemoveItem` (`self.TargetActors`) TargetActor)
  (return))

(fn `SetTargetActor`
  (params (TargetActor :type "Actor Object Reference"))
  (set `/Game/Buildings/Turret/BP_Turret.CurrantTarget` TargetActor (`self.As BP Turret`))
  (`BlackboardComponent.SetValueAsObject` (`self.Blackboard`) "CurrantTarget" TargetActor)
  (return))

(fn `UserConstructionScript`)