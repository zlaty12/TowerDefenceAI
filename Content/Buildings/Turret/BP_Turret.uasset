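; BP_Turret is an AI-driven turret that aims its cannon at a target actor and fires bullets.
; Combat-state calls toggle aiming between Idel and Combat, mirror the state to the Blackboard and reset cannon rotation on leaving combat.
; While aiming, Tick turns the cannon toward the target, with a Delay pacing BP_Bullet spawns at 0.2-second intervals.
; Target assignment is absent here, and the target-selection function only returns false.
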(event `self.ReceiveBeginPlay`
  (set `self.BlackBord` (`AIBlueprintHelperLibrary.GetBlackboard` null))
  (set `self.CanonnneutralPosition` (`self.CurrantTargetLocation`)))

(event `self.ReceiveTick`
  (params (DeltaSeconds :type "Float (single-precision)"))
  (bind _cannon (`self.CAnnon`))
  (bind _curranttarget (`self.CurrantTarget`)
    (:`then`
      (set `self.CurrantTargetLocation` (`self.K2_GetActorLocation` _curranttarget))
      (if (`self.IsAiming`)
        (`SceneComponent.K2_SetWorldRotation` _cannon (`KismetMathLibrary.FindLookAtRotation` (`SceneComponent.K2_GetComponentLocation` _cannon) (`self.CurrantTargetLocation`)) false false)
        (`KismetSystemLibrary.Delay` 0.2)
        (`|SpawnActorFromClass` "/Game/Buildings/Turret/BP_Bullet.BP_Bullet_C" (`SceneComponent.K2_GetComponentToWorld` (`self.Arrow1`)) "Undefined" "MultiplyWithRoot" null null)))
    (:`else`)))

(event `StartCombatState`
  (if (not (`self.IsAiming`))
    (set `self.IsAiming` true)))

(event `IdelState`
  (set `self.IsAiming` false))

(event `/Game/Buildings/Turret/Behavior/BPI_BehaviourTurret.NPC_Turret_set_Combat_state`
  (params (CombatState :type Boolean))
  (switch `/Game/Buildings/Turret/Behavior/E_TurretState` (`self.TurretState`)
    (:`NewEnumerator0`
      (if CombatState
        (bind _output_get (set `self.TurretState` "NewEnumerator1"))
        (`BlackboardComponent.SetValueAsEnum` (`self.BlackBord`) "TurretState" _output_get)
        (`self.StartCombatState`)))
    (:`NewEnumerator1`
      (if (not CombatState)
        (bind _output_get_2 (set `self.TurretState` "NewEnumerator0"))
        (`BlackboardComponent.SetValueAsEnum` (`self.BlackBord`) "TurretState" _output_get_2)
        (`self.IdelState`)
        (`SceneComponent.K2_SetWorldRotation` (`self.CAnnon`) (`KismetMathLibrary.Conv_VectorToRotator` (`self.CanonnneutralPosition`)) false false)))))

(fn `Controller_TurretSelectTarget`
  (returns (IsTargetSet :type Boolean))
  (return false))

(fn `UserConstructionScript`)