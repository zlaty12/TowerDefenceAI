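; BP_Base is an AI actor with health, a floating health bar widget and a currency reward on death.
; Tick pushes the current health fraction to the WB_EnemyHealth progress bar every frame.
; AnyDamage lowers and clamps health; at zero it adds currency to BP_GridManager, prints the total, destroys the actor, then calls OnDestroyed.
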(event `self.ReceiveTick`
  (params (DeltaSeconds :type "Float (single-precision)"))
  (bind _aswb_enemy_health (cast `/Game/AI/WB_EnemyHealth` (`WidgetComponent.GetWidget` (`self.Widget_HealthBar`))))
  (`ProgressBar.SetPercent` (`/Game/AI/WB_EnemyHealth.HealthBar` _aswb_enemy_health) (/ (`self.Currant Health`) (`self.Max Health`))))

(event `self.ReceiveAnyDamage`
  (params (Damage :type "Float (single-precision)") (DamageType :type "DamageType Object Reference") (InstigatedBy :type "Controller Object Reference") (DamageCauser :type "Actor Object Reference"))
  (bind _output_get (set `self.Currant Health` (`KismetMathLibrary.FClamp` (- (`self.Currant Health`) Damage) 0.0 (`self.Max Health`))))
  (if (== _output_get 0.0)
    (bind _returnvalue (`GameplayStatics.GetActorOfClass` "/Game/GridAndBuildings/Grid/BP_GridManager.BP_GridManager_C"))
    (bind _output_get_2 (set `GridManager.Curancy` (+ (`GridManager.Curancy` _returnvalue) 5.0) _returnvalue))
    (`KismetSystemLibrary.PrintString` (`KismetStringLibrary.Conv_DoubleToString` _output_get_2))
    (`self.K2_DestroyActor`)
    (`self.On Destroyed`)))

(fn `UserConstructionScript`)