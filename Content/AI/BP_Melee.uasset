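; BP_Melee is an AI melee unit pawn that chases BP_UnitNPC actors and runs a placeholder attack on targets in range.
; Tick gathers every BP_UnitNPC and issues AI MoveTo toward each in turn, every frame.
; AttackBox overlaps track actors matching ClassToDamage and start a delayed damage loop that repeats while any remain.
; DamageActor only prints debug text per overlapped actor, applying no damage.
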(event `self.ReceiveTick`
  (params (DeltaSeconds :type "Float (single-precision)"))
  (`parent.ReceiveTick` DeltaSeconds)
  (bind _outactors (`GameplayStatics.GetAllActorsOfClass` "/Game/Buildings/UnitBuilding/BP_UnitNPC.BP_UnitNPC_C"))
  (bind _output_get (set `self.AllEnemyClasses` _outactors))
  (for _array_element _output_get
    (`|AIMoveTo` self (0.0 0.0 0.0) _array_element)))

(event `DamageOverlaped actor`
  (`KismetSystemLibrary.Delay` 1.2)
  (`self.DamageActor` :!label _label)
  (`KismetSystemLibrary.Delay` 1.2)
  (if (> (`KismetArrayLibrary.Array_Length` (`self.Overlaped Actors`)) 0)
    (`KismetSystemLibrary.PrintString` "Hello")
    (goto _label)))

(event `self.AttackBox.OnComponentBeginOverlap`
  (params (OverlappedComponent :type "PrimitiveComponent Object Reference") (OtherActor :type "Actor Object Reference") (OtherComp :type "PrimitiveComponent Object Reference") (OtherBodyIndex :type Integer) (bFromSweep :type Boolean) (SweepResult :type "HitResult Structure (by ref)"))
  (if (`KismetArrayLibrary.Array_Contains` (`self.ClassToDamage`) (`GameplayStatics.GetObjectClass` OtherActor))
    (`KismetArrayLibrary.Array_Add` (`self.Overlaped Actors`) OtherActor)
    (`self.DamageOverlaped actor`)))

(event `self.AttackBox.OnComponentEndOverlap`
  (params (OverlappedComponent :type "PrimitiveComponent Object Reference") (OtherActor :type "Actor Object Reference") (OtherComp :type "PrimitiveComponent Object Reference") (OtherBodyIndex :type Integer))
  (if (`KismetArrayLibrary.Array_Contains` (`self.ClassToDamage`) (`GameplayStatics.GetObjectClass` OtherActor))
    (`KismetArrayLibrary.Array_RemoveItem` (`self.Overlaped Actors`) OtherActor)))

(fn `DamageActor`
  (for _ (`self.Overlaped Actors`)
    (`KismetSystemLibrary.PrintString` "Damaged"))
  (return))

(fn `UserConstructionScript`
  (`parent.UserConstructionScript`))