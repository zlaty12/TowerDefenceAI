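; BP_Range is an AI Blueprint, apparently a ranged variant, that is mostly a stub.
; Attack prints a debug string and plays a 2D weapon-fire sound, while Advance and Retreat are empty.
; Tick only calls the parent.
; HandleSight compares the stimulus's sense class to AISenseConfig_Sight, a config class rather than a sense class, and takes no action either way.
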(event `self.ReceiveTick`
  (params (DeltaSeconds :type "Float (single-precision)"))
  (`parent.ReceiveTick` DeltaSeconds))

(event `/Game/AI/BI_Combat.Advance`)

(event `/Game/AI/BI_Combat.Retreat`)

(event `/Game/AI/BI_Combat.Attack`
  (`KismetSystemLibrary.PrintString` "Attack")
  (`GameplayStatics.PlaySound2D` "/Game/FPWeapon/Audio/FirstPersonTemplateWeaponFire02.FirstPersonTemplateWeaponFire02" 1.0 1.0 0.0 null null))

(fn `HandleSight`
  (params (Actor :type "Actor Object Reference") (Stimulus :type "AIStimulus Structure"))
  (bind _returnvalue (`AIPerceptionSystem.GetSenseClassForStimulus` Stimulus))
  (if (not (== _returnvalue "/Script/AIModule.AISenseConfig_Sight"))
    (return)))

(fn `UserConstructionScript`
  (`parent.UserConstructionScript`))