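; BP_CameraPawn is a pawn that passes a key press on to the level's grid manager.
; BeginPlay caches all BP_FirstPersonCharacter actors and the BP_GridManager, and pressing 1 calls Switch on that manager.
; An unconnected chain, which never runs, would possess the first-person characters with player controller 0 and add the IMC_FPS mapping context through BP_TDPlayerController.
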(event `self.ReceiveBeginPlay`
  (bind _outactors (`GameplayStatics.GetAllActorsOfClass` "/Game/FirstPerson/Blueprints/BP_FirstPersonCharacter.BP_FirstPersonCharacter_C"))
  (set `self.FirstPersonChar` _outactors)
  (bind _returnvalue (`GameplayStatics.GetActorOfClass` "/Game/GridAndBuildings/Grid/BP_GridManager.BP_GridManager_C"))
  (set `self.Grid` _returnvalue))

(event `Key|One`
  (params (Key :type "Key Structure"))
  (:`Pressed`
    (`/Game/GridAndBuildings/Grid/BP_GridManager.Switch` (`self.Grid`))))

(fn `UserConstructionScript`)